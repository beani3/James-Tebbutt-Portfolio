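; Enemy AI character that takes random damage from first-person projectile hits and can drop a pickup on death.
; Each hit lowers health and calls DestroyEnemy, which destroys the actor and flags it dead once health runs out.
; Death increases the score on the guide game mode, then spawns either health or, more often, ammo.
; Drops are capped by an ammo pickup count cached at BeginPlay, not the live count.
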(event EventBeginPlay
  (bind _asbp_guide_game_mode (Utilities|Casting|CastToBP_Guide_GameMode (Game|GetGameMode)))
  (Variables|Default|SetAs%20BP%20Guide%20Game%20Mode _asbp_guide_game_mode)
  (bind _outactors (Actor|GetAllActorsOfClass "/Game/FirstPerson/Blueprints/BP_Ammo_Pickup.BP_Ammo_Pickup_C"))
  (Variables|Default|SetOut%20Actors _outactors))

(event Collision|EventActorBeginOverlap
  (params (OtherActor :type Actor%20Object%20Reference)))

(event EventTick
  (params (DeltaSeconds :type Float%20%28single-precision%29)))

(event Collision|EventHit
  (params (MyComp :type Primitive%20Component%20Object%20Reference) (Other :type Actor%20Object%20Reference) (OtherComp :type Primitive%20Component%20Object%20Reference) (bSelfMoved :type Boolean) (HitLocation :type Vector :default "0, 0, 0") (HitNormal :type Vector :default "0, 0, 0") (NormalImpulse :type Vector :default "0, 0, 0") (Hit :type Hit%20Result%20Structure%20%28by%20ref%29))
  (Utilities|Casting|CastToBP_FirstPersonProjectile Other)
  (Variables|Default|SetEnemyHealth (- (Variables|Default|GetEnemyHealth) (Math|Random|RandomFloatinRange 5.0 1e+01)))
  (CallFunction|DestroyEnemy)
  (if (== (Variables|Default|GetbEnemyDead) true)
    (Default|IncreaseScore (Variables|Default|GetAs%20BP%20Guide%20Game%20Mode))
    (if (< (Utilities|Array|Length (Variables|Default|GetOut%20Actors)) 10)
      (if (== (Math|Random|RandomIntegerinRange 0 4) 0)
        (Game|SpawnActorfromClass "/Game/FirstPerson/Blueprints/BP_Health_Pickup.BP_Health_Pickup_C" (Transformation|GetActorTransform) "Undefined" "MultiplyWithRoot" 0 0)
        (else
          (Game|SpawnActorfromClass "/Game/FirstPerson/Blueprints/BP_Ammo_Pickup.BP_Ammo_Pickup_C" (Transformation|GetActorTransform) "Undefined" "MultiplyWithRoot" 0 0))))))

(fn ConstructionScript)

(fn DestroyEnemy
  (if (<= (Variables|Default|GetEnemyHealth) 0.0)
    (Development|PrintString "Enemy Died!")
    (Actor|DestroyActor)
    (Variables|Default|SetbEnemyDead true)))