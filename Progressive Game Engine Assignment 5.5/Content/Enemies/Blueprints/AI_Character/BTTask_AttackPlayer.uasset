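; Behavior tree task that sends an enemy pawn after the player and damages them on arrival.
; Records the player's location on the blackboard, then runs AIMoveTo on the player character.
; On success it applies fixed damage and subtracts the returned amount from Health on BP_Guide_GameMode, caching that cast.
; The task finishes only on that success path; a failed move or cast never calls FinishExecute.
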(event EventReceiveExecuteAI
  (params (OwnerController :type AI%20Controller%20Object%20Reference) (ControlledPawn :type Pawn%20Object%20Reference))
  (bind _returnvalue (Game|GetPlayerCharacter 0))
  (bind _returnvalue_2 (Transformation|GetActorLocation _returnvalue))
  (AI|BehaviorTree|SetBlackboardValueasVector (Variables|Default|GetPlayerLocationVector) _returnvalue_2)
  (AI|AIMoveTo ControlledPawn _returnvalue_2 _returnvalue 0.0 true
    (:OnSuccess
      (bind _returnvalue_3 (Game|Damage|ApplyDamage _returnvalue 5.0 0 0))
      (Utilities|IsValid (Variables|Default|GetAs%20BP%20Guide%20Game%20Mode)
        (:Is%20Valid
          _)
        (:Is%20Not%20Valid
          (bind _asbp_guide_game_mode (Utilities|Casting|CastToBP_Guide_GameMode (Game|GetGameMode)))
          (bind _output_get (Variables|Default|SetAs%20BP%20Guide%20Game%20Mode _asbp_guide_game_mode))))
      (Variables|/Game/Guide/BP_Guide_GameMode.BP_Guide_GameMode_C|SetHealth _output_get (- (Variables|/Game/Guide/BP_Guide_GameMode.BP_Guide_GameMode_C|GetHealth (Variables|Default|GetAs%20BP%20Guide%20Game%20Mode)) _returnvalue_3))
      (AI|BehaviorTree|FinishExecute true))))