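; Game mode for a guide shooter project that holds health, ammo, magazines and score and shows the HUD and game-over screen.
; BeginPlay resets stats through StartGame and creates the UI widget.
; Simple functions handle pickups, ammo use, reloads and random score gains.
; Tick pushes stats into the HUD and runs the game-over check, which adds the end widget and switches to UI-only input when health runs out.
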(event Custom|GameOverEvent
  (bind _returnvalue (Game|GetPlayerController 0))
  ;[1 0.5544 0.04048] Game Over Logic
  (if (<= (Variables|Default|GetHealth) (Variables|Default|GetnulHealth))
    (Variables|Default|SetGameOver true)
    (bind _returnvalue_2 (Game|ConstructObjectfromClass "/Game/Menus/WB_GameOver.WB_GameOver_C"))
    (UserInterface|Viewport|AddtoViewport _returnvalue_2 0)
    (Input|SetInputModeUIOnly _returnvalue (Variables|Default|GetGameOverRef) "DoNotLock" false)
    (Variables|/Script/Engine.PlayerController|SetbShowMouseCursor _returnvalue true)
    (else
      ;[0.1927 1 0.4548] Sets the UI variables
      (Variables|/Game/UI/WB_MyUI.WB_MyUI_C|SetMagVar (Variables|Default|GetUIRef) (* (Variables|Default|GetMags) 20))
      (Variables|/Game/UI/WB_MyUI.WB_MyUI_C|SetScoreVar (Variables|Default|GetUIRef) (Variables|Default|GetScore))
      (Variables|/Game/UI/WB_MyUI.WB_MyUI_C|SetHealthVar (Variables|Default|GetUIRef) (Variables|Default|GetHealth)))))

(event EventBeginPlay
  ;[0.1623 0.9219 0.1584] Creates the UI widget upon game start
  (Development|PrintString "Start Game")
  (Utilities|StartGame
    (:Out
      (Utilities|IsValid (Variables|Default|GetUIRef)
        (:Is%20Valid
          _)
        (:Is%20Not%20Valid
          (bind _returnvalue (UserInterface|CreateWidget "/Game/UI/WB_MyUI.WB_MyUI_C" (Game|GetPlayerController 0)))
          (bind _output_get (Variables|Default|SetUIRef _returnvalue))))
      (Widget|SetFocus _output_get)
      (UserInterface|Viewport|AddtoViewport _output_get 0))))

(event EventTick
  (params (DeltaSeconds :type Float%20%28single-precision%29))
  (bind _returnvalue (Game|GetPlayerController 0))
  ;[0.1927 1 0.4548] Sets the UI variables
  (Variables|/Game/UI/WB_MyUI.WB_MyUI_C|SetAmmoVar (Variables|Default|GetUIRef) (Variables|Default|GetAmmo))
  ;[1 0.5544 0.04048] Game Over Logic
  (if (<= (Variables|Default|GetHealth) (Variables|Default|GetnulHealth))
    (Variables|Default|SetGameOver true)
    (bind _returnvalue_2 (Game|ConstructObjectfromClass "/Game/Menus/WB_GameOver.WB_GameOver_C"))
    (UserInterface|Viewport|AddtoViewport _returnvalue_2 0)
    (Input|SetInputModeUIOnly _returnvalue (Variables|Default|GetGameOverRef) "DoNotLock" false)
    (Variables|/Script/Engine.PlayerController|SetbShowMouseCursor _returnvalue true)
    (else
      (Variables|/Game/UI/WB_MyUI.WB_MyUI_C|SetMagVar (Variables|Default|GetUIRef) (* (Variables|Default|GetMags) 20))
      (Variables|/Game/UI/WB_MyUI.WB_MyUI_C|SetScoreVar (Variables|Default|GetUIRef) (Variables|Default|GetScore))
      (Variables|/Game/UI/WB_MyUI.WB_MyUI_C|SetHealthVar (Variables|Default|GetUIRef) (Variables|Default|GetHealth)))))

(fn ConstructionScript)

(fn AmmoCollected
  ;[0.2188 1 0.3563] Ammo Collectable Logic
  (Variables|Default|SetAmmo (+ (Variables|Default|GetAmmo) 5)))

(fn UseAmmo
  ;[0 1 0.2888] Ammo Use Logic
  (Variables|Default|SetAmmo (- (Variables|Default|GetAmmo) 1)))

(fn Reload
  ;[0 1 0.0137] Reload Logic
  (Variables|Default|SetAmmo 20)
  (Variables|Default|SetMags (- (Variables|Default|GetMags) 1)))

(fn IncreaseScore
  ;[0 1 0.2671] Scoring System Logic
  (Variables|Default|SetScore (+ (Variables|Default|GetScore) (Math|Random|RandomIntegerinRange 100 200))))

(fn HealthCollected
  ;[0.2652 1 0.2292] Health Collectable Logic
  (Variables|Default|SetHealth (+ (Variables|Default|GetHealth) 1e+01)))